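; BP_PillarGroup is a puzzle controller that opens a linked door once every pillar in its group has been hit.
; On BeginPlay it binds a handler to each pillar's sword-hit dispatcher.
; Each hit event recounts the pillars flagged as hit and calls OpenDoor on the linked door when the count equals the array length.
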(event Custom|PillarHasBeenHit
  (Variables|Default|SetnbHit 0)
  (bind _array_element (Utilities|Array|ForEachLoopwithBreak (Variables|Default|GetPillars))
    (:LoopBody
      (if (Variables|/Game/01-Blueprints/BP_Pillar.BP_Pillar_C|GetHasBeenHit _array_element)
        (bind _result (Math|Integer|IncrementInt (Variables|Default|GetnbHit))
          (:%20%20
            (Variables|Default|SetnbHit _result)))))
    (:Completed
      (if (== (Variables|Default|GetnbHit) (Utilities|Array|Length (Variables|Default|GetPillars)))
        (Default|OpenDoor (Variables|Default|GetLinkDoor))))))

(event EventBeginPlay
  (for _array_element (Variables|Default|GetPillars)
    (EventDispatchers|AssignPillarSwordHit _array_element (delegate Custom|PillarHasBeenHit))))

(fn ConstructionScript)