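; BP_BaseBallLauncher is a baseball launcher that swings an arm and throws balls until a maximum count is reached.
; After a delay on BeginPlay, the RotateBras timeline drives the arm pivot's pitch.
; A timeline event track hides the visible fake ball, spawns a BP_BaseBall_Ball at the spawner transform and increments the count.
; When the timeline finishes, the fake ball reappears and the swing replays if balls remain.
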(event Custom|RotateBrasPivot
  (bind _rotatepitch (Timeline|RotateBras PlayFromStart)
    (:Update
      (Transformation|SetRelativeRotation (Variables|Default|GetBrasPivot) (Math|Rotator|MakeRotator 0.0 _rotatepitch 0.0) false false))
    (:Finished
      (Development|SetHiddeninGame (Variables|Default|GetFakeBall) false false)
      (CallFunction|CanReplay?))
    (:SpawnProjectile
      (CallFunction|SpawnBallProjectile))))

(event Custom|SpawnBallProjectile
  (Development|SetHiddeninGame (Variables|Default|GetFakeBall) true false)
  (Game|SpawnActorfromClass "/Game/01-Blueprints/BaseBall/BP_BaseBall_Ball.BP_BaseBall_Ball_C" (Transformation|GetWorldTransform (Variables|Default|GetProjectileSpawner2)) "AlwaysSpawn" "MultiplyWithRoot" 0 0)
  (Math|Integer|IncrementInt (Variables|Default|GetCurrentSpawnBall)))

(event Custom|CanReplay?
  (if (< (Variables|Default|GetCurrentSpawnBall) (Variables|Default|GetMaxNumberSpawnBall))
    (CallFunction|RotateBrasPivot)))

(event EventBeginPlay
  (Utilities|FlowControl|Delay 5.0)
  (CallFunction|RotateBrasPivot))

(fn ConstructionScript)