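; BP_Piedestal is a pedestal that accepts a master key item and opens its linked door when that key matches.
; When a key overlaps the sphere and the slot is empty, it releases the grab and snaps the key to ItemPos with physics paused for one second.
; It compares the stored key to the door's KeyToOpen by reference.
; Any master key leaving the sphere clears the slot, without closing the door.
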(event OnComponentBeginOverlap(Sphere)
  (params (OverlappedComponent :type Primitive%20Component%20Object%20Reference) (OtherActor :type Actor%20Object%20Reference) (OtherComp :type Primitive%20Component%20Object%20Reference) (OtherBodyIndex :type Integer) (bFromSweep :type Boolean) (SweepResult :type Hit%20Result%20Structure%20%28by%20ref%29))
  (bind _asbp_item_master_key (Utilities|Casting|CastToBP_Item_MasterKey OtherActor))
  (Utilities|IsValid (Variables|Default|GetItemDroppedOnpiedestal)
    (:Is%20Not%20Valid
      (Variables|Default|SetItemDroppedOnpiedestal _asbp_item_master_key)
      (Default|TryRelease (Variables|/Game/01-Blueprints/BP_MasterItem.BP_MasterItem_C|GetGrabComponent _asbp_item_master_key))
      (Default|CallOnDropped (Variables|/Game/01-Blueprints/BP_MasterItem.BP_MasterItem_C|GetGrabComponent _asbp_item_master_key))
      (Physics|SetSimulatePhysics (Variables|/Game/01-Blueprints/BP_MasterItem.BP_MasterItem_C|GetMesh _asbp_item_master_key) false)
      (Transformation|SetActorLocationAndRotation _asbp_item_master_key (Transformation|GetWorldLocation (Variables|Default|GetItemPos)) "0, 0, 0" false true)
      (Utilities|FlowControl|Sequence
        (:then_0
          (CallFunction|CheckItemtoOpenDoor))
        (:then_1
          (Utilities|FlowControl|Delay 1.0)
          (Physics|SetSimulatePhysics (Variables|/Game/01-Blueprints/BP_MasterItem.BP_MasterItem_C|GetMesh _asbp_item_master_key) true))))))

(event OnComponentEndOverlap(Sphere)
  (params (OverlappedComponent :type Primitive%20Component%20Object%20Reference) (OtherActor :type Actor%20Object%20Reference) (OtherComp :type Primitive%20Component%20Object%20Reference) (OtherBodyIndex :type Integer))
  (Utilities|Casting|CastToBP_Item_MasterKey OtherActor)
  (Utilities|IsValid (Variables|Default|GetItemDroppedOnpiedestal)
    (:Is%20Valid
      (Variables|Default|SetItemDroppedOnpiedestal 0))))

(event Custom|CheckItemToOpenDoor
  (bind _linkdoor (Variables|Default|GetLinkDoor))
  (bind _keytoopen (Variables|/Game/01-Blueprints/BP_Door.BP_Door_C|GetKeyToOpen _linkdoor))
  (Utilities|IsValid _linkdoor
    (:Is%20Valid
      (Utilities|IsValid _keytoopen
        (:Is%20Valid
          (if (== _keytoopen (Variables|Default|GetItemDroppedOnpiedestal))
            (Default|OpenDoor (Variables|Default|GetLinkDoor))))))))

(fn ConstructionScript)