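; BP_TestSword is a test sword that cuts procedural meshes it hits when swung fast enough.
; Tick measures the static mesh's speed from its change in world position each frame.
; Box hits above a speed threshold slice the mesh at the impact point along the sword's right vector, capping the cut and launching the new half with physics.
; A short delayed flag reset prevents repeated slices.
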(event OnComponentHit(Box)
  (params (HitComponent :type Primitive%20Component%20Object%20Reference) (OtherActor :type Actor%20Object%20Reference) (OtherComp :type Primitive%20Component%20Object%20Reference) (NormalImpulse :type Vector :default "0, 0, 0") (Hit :type Hit%20Result%20Structure%20%28by%20ref%29))
  ;[0.15 0.15 0.15 0.5] Gestion du slice mesh
  (bind _asprocedural_mesh_component (Utilities|Casting|CastToProceduralMeshComponent OtherComp))
  (if (not (Variables|Default|GetHasBeenSliced))
    (if (> (Variables|Default|GetSpeed) 5e+02)
      (bind _outotherhalfprocmesh (Class|KismetProceduralMeshLibrary|SliceProceduralMesh _asprocedural_mesh_component (.Location (Collision|BreakHitResult Hit)) (Math|Vector|GetRightVector (Variables|Default|GetStaticMesh)) true "CreateNewSectionForCap" "/Game/FPWeapon/Materials/BaseMaterial.BaseMaterial"))
      (Physics|SetSimulatePhysics _outotherhalfprocmesh true)
      (Physics|AddImpulse _outotherhalfprocmesh "100.000000,100.000000,100.000000" "None" true)
      (Variables|Default|SetHasBeenSliced true)
      (Utilities|FlowControl|Delay 0.3)
      (Variables|Default|SetHasBeenSliced false))))

(event Custom|SetDistanceMoved
  ;[0.15 0.15 0.15 0.5] Calcul de la distance depuis la derniere position
  (bind _output_get (Variables|Default|SetCurrent%20pos (Transformation|GetWorldLocation (Variables|Default|GetStaticMesh))))
  (bind _output_get_2 (Variables|Default|SetDistance%20moved (Math|Vector|VectorLength (- _output_get (Variables|Default|GetLastPos)))))
  (Variables|Default|SetLastPos _output_get))

(event EventBeginPlay)

(event Collision|EventActorBeginOverlap
  (params (OtherActor :type Actor%20Object%20Reference)))

(event EventTick
  (params (DeltaSeconds :type Float%20%28single-precision%29))
  ;[0.15 0.15 0.15 0.5] Calcul de la vitesse de l'objet
  (CallFunction|SetDistanceMoved)
  (Variables|Default|SetSpeed (/ (Variables|Default|GetDistance%20moved) DeltaSeconds)))

(fn ConstructionScript)