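; BP_Screen is an in-game display actor that shows ball count, ball distance and the maximum distance reached.
; Two events receive new count and distance values and write them to their text components.
; The distance event also tracks the largest value received, updating the max-distance text only when that record is beaten.
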(event Custom|SetBallCount_Event
  (params (Count :type Integer))
  (Rendering|Components|TextRender|SetText (Variables|Default|GetTextBallCount) (Utilities|Text|ToText(Integer) Count)))

(event Custom|SetBallDistance_Event
  (params (BallDistance :type Float%20%28double-precision%29))
  (Rendering|Components|TextRender|SetText (Variables|Default|GetTextBallDistance) (Utilities|Text|ToText(Float) BallDistance "HalfToEven"))
  (if (> BallDistance (Variables|Default|GetMaxDistance))
    (bind _output_get (Variables|Default|SetMaxDistance BallDistance))
    (Rendering|Components|TextRender|SetText (Variables|Default|GetTextMaxDistance) (Utilities|Text|ToText(Float) _output_get "HalfToEven"))))

(fn ConstructionScript)