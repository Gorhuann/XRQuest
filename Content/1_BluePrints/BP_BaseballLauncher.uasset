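; Baseball launcher Blueprint that pitches a round of ten balls, showing the count and END on text and reporting to a screen.
; A timeline, sped up by difficulty, swings the arm and swaps the fake ball for a spawned physics ball with difficulty-scaled velocity.
; Tick reports the ball's distance and destroys it when slow; destruction, also triggered by lifespan expiry, chains the next delayed launch.
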(event Custom|RotateArm_Event
  (bind _rotation (Timeline|Timeline PlayFromStart)
    (:Update
      (Transformation|SetRelativeRotation (Variables|Default|GetJoint) (Math|Rotator|MakeRotator 0.0 _rotation 0.0) false false))
    (:Finished
      (Development|SetHiddeninGame (Variables|Default|GetFakeBall) false false))
    (:SpawnBall
      (CallFunction|SpawnBallEvent))))

(event Custom|SpawnBall_Event
  (Development|SetHiddeninGame (Variables|Default|GetFakeBall) true false)
  (bind _returnvalue (Game|SpawnActorfromClass (Variables|Default|GetBall) (Transformation|GetWorldTransform (Variables|Default|GetBallSpawnPoint)) "AlwaysSpawn" "MultiplyWithRoot" 0 0))
  (bind _output_get (Variables|Default|SetCurrentBall _returnvalue))
  (Class|PrimitiveComponent|SetAllPhysicsLinearVelocity (Variables|/Game/1_BluePrints/BP_Ball.BP_Ball_C|GetBall _output_get) (* "-1.000000,0.000000,0.100000" (* (Variables|Default|GetInitial%20Speed) (Variables|Default|GetDifficulty))) false)
  (Actor|SetLifeSpan _returnvalue 1e+01)
  (Game|AssignOnDestroyed _returnvalue (delegate Custom|OnDestroyed_Event)))

(event Custom|StartGame_Event
  (params (Difficulty :type Float%20%28double-precision%29))
  (if (or (>= (Variables|Default|Getindex) 10) (<= (Variables|Default|Getindex) 0))
    (Variables|Default|SetDifficulty Difficulty)
    (Components|Timeline|SetPlayRate (Variables|Default|GetTimeline) Difficulty)
    (Variables|Default|Setindex 0)
    (CallFunction|LaunchBallEvent)))

(event Custom|LaunchBall_Event
  (bind _textscore (Variables|Default|GetTextScore))
  (bind _textrender (Variables|/Script/Engine.TextRenderActor|GetTextRender _textscore))
  (if (< (Variables|Default|Getindex) 10)
    (Variables|Default|Setindex (+ (Variables|Default|Getindex) 1))
    (Utilities|FlowControl|Delay 4.0)
    (Rendering|Components|TextRender|SetText _textrender (Utilities|Text|ToText(Integer) (Variables|Default|Getindex)))
    (Default|SetBallCountEvent (Variables|Default|GetScreen) (Variables|Default|Getindex))
    (CallFunction|RotateArmEvent)
    (if (>= (Variables|Default|Getindex) 10)
      (Rendering|Components|TextRender|SetText _textrender (Utilities|Text|ToText(String) "END")))))

(event Custom|OnDestroyed_Event
  (params (DestroyedActor :type Actor%20Object%20Reference))
  (CallFunction|LaunchBallEvent))

(event EventTick
  (params (DeltaSeconds :type Float%20%28single-precision%29))
  (bind _currentball (Variables|Default|GetCurrentBall))
  (bind _ball (Variables|/Game/1_BluePrints/BP_Ball.BP_Ball_C|GetBall _currentball))
  (if (Utilities|IsValid _currentball)
    (bind _returnvalue (Physics|GetPhysicsLinearVelocity _ball "None"))
    (if (<= (Math|Vector|VectorLength _returnvalue) 1e+02)
      (Actor|DestroyActor (Variables|Default|GetCurrentBall))
      (else
        (Default|SetBallDistanceEvent (Variables|Default|GetScreen) (Math|Vector|Distance(Vector) (Transformation|GetWorldLocation _ball) (Transformation|GetWorldLocation (Variables|/Script/Engine.Actor|GetRootComponent (Variables|Default|GetBase)))))))))

(fn ConstructionScript)