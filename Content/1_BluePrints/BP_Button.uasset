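; BP_Button is a pressable button that reacts when a VRPawn overlaps its Box trigger.
; On overlap it disables the box's overlap events, animates the Sphere down along Z and calls ButtonPress to signal the press.
; After a short delay it moves the Sphere back to the height cached at BeginPlay and re-enables overlaps, preventing retriggers mid-animation.
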(event OnComponentBeginOverlap(Box)
  (params (OverlappedComponent :type Primitive%20Component%20Object%20Reference) (OtherActor :type Actor%20Object%20Reference) (OtherComp :type Primitive%20Component%20Object%20Reference) (OtherBodyIndex :type Integer) (bFromSweep :type Boolean) (SweepResult :type Hit%20Result%20Structure%20%28by%20ref%29))
  (bind _sphere (Variables|Default|GetSphere))
  (bind _sphere_2 (Variables|Default|GetSphere))
  (bind _relativelocation (Variables|/Script/Engine.SceneComponent|GetRelativeLocation _sphere_2))
  (Utilities|Casting|CastToVRPawn OtherActor)
  (Variables|/Script/Engine.PrimitiveComponent|SetbGenerateOverlapEvents (Variables|Default|GetBox) false)
  (Components|MoveComponentTo _sphere (- (Variables|/Script/Engine.SceneComponent|GetRelativeLocation _sphere) "0.000000,0.000000,100.000000") "0, 0, 0" false false 0.2 false)
  (Default|CallButtonPress)
  (Utilities|FlowControl|Delay 0.1)
  (Components|MoveComponentTo (Variables|Default|GetSphere) (Math|Vector|MakeVector (.x _relativelocation) (.y _relativelocation) (Variables|Default|GetButtonStartZ)) "0, 0, 0" false false 0.2 false)
  (Variables|/Script/Engine.PrimitiveComponent|SetbGenerateOverlapEvents (Variables|Default|GetBox) true))

(event EventBeginPlay
  (Variables|Default|SetButtonStartZ (.z (Variables|/Script/Engine.SceneComponent|GetRelativeLocation (Variables|Default|GetSphere)))))

(fn ConstructionScript)