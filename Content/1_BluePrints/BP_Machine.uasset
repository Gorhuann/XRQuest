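; BP_Machine is a control machine that starts a game event on a left or right thrower at an adjustable difficulty.
; On BeginPlay it binds four in-world buttons for start, side switch and difficulty up or down, with Space Bar as an alternate start trigger.
; Side and difficulty changes update text displays, difficulty is stepped within a clamped range, and start passes it to the selected thrower.
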(event Custom|SwitchSide
  (CallFunction|PressSwitchSide))

(event Custom|IncreaseDifficulty
  (CallFunction|PressIncreaseDifficulty))

(event Custom|Start
  (CallFunction|PressStart))

(event Custom|DecreaseDifficulty
  (CallFunction|PressDecreaseDifficulty))

(event EventBeginPlay
  (EventDispatchers|AssignButtonPress (Variables|Default|GetButtonStart) (delegate Custom|Start))
  (EventDispatchers|AssignButtonPress (Variables|Default|GetButtonSwitchSide) (delegate Custom|SwitchSide))
  (EventDispatchers|AssignButtonPress (Variables|Default|GetButtonIncreaseDifficulty) (delegate Custom|IncreaseDifficulty))
  (EventDispatchers|AssignButtonPress (Variables|Default|GetButtonDecreaseDifficulty) (delegate Custom|DecreaseDifficulty)))

(event Input|KeyboardEvents|SpaceBar
  (params (Key :type Key%20Structure :default "None"))
  (:Pressed
    (CallFunction|PressStart)))

(fn ConstructionScript)

(fn PressStart
  (bind _difficulty (Variables|Default|GetDifficulty))
  (if (Variables|Default|GetIsLeft)
    (Default|StartGameEvent (Variables|Default|GetLeftThrower) _difficulty)
    (else
      (Default|StartGameEvent (Variables|Default|GetRightThrower) _difficulty))))

(fn PressSwitchSide
  (bind _output_get (Variables|Default|SetIsLeft (not (Variables|Default|GetIsLeft))))
  (if _output_get
    (Rendering|Components|TextRender|SetText (Variables|/Script/Engine.TextRenderActor|GetTextRender (Variables|Default|GetSideText)) (Utilities|Text|ToText(String) "LEFT"))
    (else
      (Rendering|Components|TextRender|SetText (Variables|/Script/Engine.TextRenderActor|GetTextRender (Variables|Default|GetSideText)) (Utilities|Text|ToText(String) "RIGHT")))))

(fn PressIncreaseDifficulty
  (bind _output_get (Variables|Default|SetDifficulty (Math|Float|Clamp(Float) (+ (Variables|Default|GetDifficulty) 0.1) 0.5 2.0)))
  (Rendering|Components|TextRender|SetText (Variables|/Script/Engine.TextRenderActor|GetTextRender (Variables|Default|GetDifficultyText)) (Utilities|Text|ToText(Float) _output_get "HalfToEven")))

(fn PressDecreaseDifficulty
  (bind _output_get (Variables|Default|SetDifficulty (Math|Float|Clamp(Float) (- (Variables|Default|GetDifficulty) 0.1) 0.5 2.0)))
  (Rendering|Components|TextRender|SetText (Variables|/Script/Engine.TextRenderActor|GetTextRender (Variables|Default|GetDifficultyText)) (Utilities|Text|ToText(Float) _output_get "HalfToEven")))